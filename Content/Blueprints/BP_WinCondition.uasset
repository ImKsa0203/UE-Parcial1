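; BP_WinCondition ends the level once every pressure plate in its Plates array is active.
; On BeginPlay it binds to each plate's activated and deactivated dispatchers to keep a running count of active plates.
; When the count reaches the array length, it sets the menu type on BP_GameInstance and opens the HP_Menu level.
; Deactivation lowers the count, and its follow-up comparison triggers nothing.
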(event Custom|DeactivatedPlate
  (bind _count (Variables|Default|GetCount))
  (Math|Integer|DecrementInt _count
    (:%20%20
      (if (== _count (- (Utilities|Array|Length (Variables|Default|GetPlates)) 1))
        _))))

(event Custom|ActivatedPlate
  (bind _count (Variables|Default|GetCount))
  (Math|Integer|IncrementInt _count
    (:%20%20
      (if (>= _count (Utilities|Array|Length (Variables|Default|GetPlates)))
        (bind _asbp_game_instance (Utilities|Casting|CastToBP_GameInstance (Game|GetGameInstance)))
        (Variables|/Game/ThirdPerson/Blueprints/BP_GameInstance.BP_GameInstance_C|SetMenuType _asbp_game_instance "NewEnumerator1")
        (Game|OpenLevel(byName) "HP_Menu")))))

(event EventBeginPlay
  (for _array_element (Variables|Default|GetPlates)
    (EventDispatchers|BindEventtoActivatedEventDispatcher _array_element (delegate Custom|ActivatedPlate))
    (EventDispatchers|BindEventtoDeactivatedEventDispatcher _array_element (delegate Custom|DeactivatedPlate))))

(fn ConstructionScript)