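; BP_PreasurePlate is a pressure plate that reacts to BP_PusheableObject actors resting on it.
; Box overlap events raise and lower a Count of those objects, filtered by exact class.
; The first object to enter fires the Activated dispatcher, and the count falling to zero fires the Deactivated dispatcher, each with a debug print.
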(event OnComponentBeginOverlap(Box)
  (params (OverlappedComponent :type Primitive%20Component%20Object%20Reference) (OtherActor :type Actor%20Object%20Reference) (OtherComp :type Primitive%20Component%20Object%20Reference) (OtherBodyIndex :type Integer) (bFromSweep :type Boolean) (SweepResult :type Hit%20Result%20Structure%20%28by%20ref%29))
  (bind _count (Variables|Default|GetCount))
  (if (== (Utilities|GetClass OtherActor) "/Game/Blueprints/BP_PusheableObject.BP_PusheableObject_C")
    (Math|Integer|IncrementInt _count
      (:%20%20
        (if (== _count 1)
          (Development|PrintString "Activated Plate" true true "(R=0.000000,G=1.000000,B=1.000000,A=1.000000)")
          (Default|CallActivatedEventDispatcher))))))

(event OnComponentEndOverlap(Box)
  (params (OverlappedComponent :type Primitive%20Component%20Object%20Reference) (OtherActor :type Actor%20Object%20Reference) (OtherComp :type Primitive%20Component%20Object%20Reference) (OtherBodyIndex :type Integer))
  (bind _count (Variables|Default|GetCount))
  (if (== (Utilities|GetClass OtherActor) "/Game/Blueprints/BP_PusheableObject.BP_PusheableObject_C")
    (Math|Integer|DecrementInt _count
      (:%20%20
        (if (<= _count 0)
          (Development|PrintString "Deactivated Plate" true true "(R=0.000000,G=0.000000,B=1.000000,A=1.000000)")
          (Default|CallDeactivatedEventDispatcher))))))

(fn ConstructionScript)