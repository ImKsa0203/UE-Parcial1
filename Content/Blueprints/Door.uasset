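; Interactable door Blueprint that toggles between open and closed, either through Interact or by a spell.
; A Timeline lerps the Pivot's relative location and rotation between open and closed transforms, reversing to open and playing forward to close.
; The construction script calls SetTime with a value chosen from IsOpen to set the initial Timeline time.
; UseSpell ignores direction, calls Interact and returns the spell name "Alohomora".
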(event Custom|Interact
  (bind _pivot (Variables|Default|GetPivot))
  (Variables|Default|SetIsOpen (not (Variables|Default|GetIsOpen)))
  (if (Variables|Default|GetIsOpen)
    (bind _lerp (Timeline|Timeline Reverse)
      (:Update
        (Transformation|SetRelativeLocation _pivot (Math|Vector|Lerp(Vector) (Variables|Default|GetOpenPosition) (Variables|Default|GetClosePosition) _lerp) false false)
        (Transformation|SetRelativeRotation _pivot (Math|Rotator|Lerp(Rotator) (Variables|Default|GetOpenRotation) (Variables|Default|GetCloseRotation) _lerp) false false)))
    (else
      (Timeline|Timeline Play))))

(event Custom|SetTime
  (params (NewTime :type Float%20%28single-precision%29))
  (bind _pivot (Variables|Default|GetPivot))
  (bind _lerp (Timeline|Timeline SetNewTime)
    (:Update
      (Transformation|SetRelativeLocation _pivot (Math|Vector|Lerp(Vector) (Variables|Default|GetOpenPosition) (Variables|Default|GetClosePosition) _lerp) false false)
      (Transformation|SetRelativeRotation _pivot (Math|Rotator|Lerp(Rotator) (Variables|Default|GetOpenRotation) (Variables|Default|GetCloseRotation) _lerp) false false))))

(fn ConstructionScript
  (CallFunction|SetTime (Math|Float|SelectFloat 0.0 1.0 (Variables|Default|GetIsOpen))))

(fn UseSpell
  (params (Direction :type Vector :default "0, 0, 0"))
  (CallFunction|Interact)
  (return "Alohomora"))