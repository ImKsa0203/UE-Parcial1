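; A platform that moves along a timeline-driven offset, with a scalable vertical fall, when the third-person character steps on it.
; Box overlaps track whether the player is on top and start the timeline, which sets the platform's relative location.
; The timeline reverses after each forward pass, then replays if the player is still aboard.
; A Reset event track jumps the timeline's time during reverse playback.
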(event OnComponentBeginOverlap(Box)
  (params (OverlappedComponent :type Primitive%20Component%20Object%20Reference) (OtherActor :type Actor%20Object%20Reference) (OtherComp :type Primitive%20Component%20Object%20Reference) (OtherBodyIndex :type Integer) (bFromSweep :type Boolean) (SweepResult :type Hit%20Result%20Structure%20%28by%20ref%29))
  (if (== (Utilities|GetClass OtherActor) "/Game/ThirdPerson/Blueprints/BP_ThirdPersonCharacter.BP_ThirdPersonCharacter_C")
    (Variables|Default|SetPlayerOnTop true)
    (CallFunction|Activate)))

(event OnComponentEndOverlap(Box)
  (params (OverlappedComponent :type Primitive%20Component%20Object%20Reference) (OtherActor :type Actor%20Object%20Reference) (OtherComp :type Primitive%20Component%20Object%20Reference) (OtherBodyIndex :type Integer))
  (if (== (Utilities|GetClass OtherActor) "/Game/ThirdPerson/Blueprints/BP_ThirdPersonCharacter.BP_ThirdPersonCharacter_C")
    (Variables|Default|SetPlayerOnTop false)))

(event Custom|Activate
  (if (not (Audio|Components|Audio|IsPlaying (Variables|Default|GetMovementTimeline)))
    (bind (_direction _movement) (Timeline|MovementTimeline PlayFromStart)
      (:Update
        (Transformation|SetRelativeLocation (Variables|Default|GetPlatform) (* _movement (Variables|Default|GetMovement) (Math|Vector|MakeVector 1.0 1.0 (Variables|Default|GetVerticalFall))) false false))
      (:Finished
        (if (Utilities|Enum|Equal(Enum) _direction "Forward")
          (Timeline|MovementTimeline ReverseFromEnd)
          (elif (Variables|Default|GetPlayerOnTop)
            (Timeline|MovementTimeline PlayFromStart))))
      (:Reset
        ;[1 1 1] Reset
        (if (Utilities|Enum|Equal(Enum) _direction "Backward")
          (Timeline|MovementTimeline SetNewTime))))))

(fn ConstructionScript)