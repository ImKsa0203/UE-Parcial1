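; BP_Projectile is a projectile that damages or sends a spell message to what it hits, and self-destructs after a timed lifetime.
; On sphere hit, it applies Damage through BPI_Damageable on the target's Comp_Health component.
; Failing that, non-door actors implementing the Spell interface receive UseSpellMessage with a scaled forward vector, and the result is debug-printed.
; Any hit on a valid actor destroys the projectile.
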(event OnComponentHit(Sphere)
  (params (HitComponent :type Primitive%20Component%20Object%20Reference) (OtherActor :type Actor%20Object%20Reference) (OtherComp :type Primitive%20Component%20Object%20Reference) (NormalImpulse :type Vector :default "0, 0, 0") (Hit :type Hit%20Result%20Structure%20%28by%20ref%29))
  (Utilities|IsValid OtherActor
    (:Is%20Valid
      (bind _asbpi_damageable (Utilities|Casting|CastToBPI_Damageable (Actor|GetComponentbyClass OtherActor "/Game/Blueprints/ActorComponents/Comp_Health.Comp_Health_C"))
        (:then
          (Default|Damage _asbpi_damageable (Variables|Default|GetDamage))
          (Actor|DestroyActor))
        (:CastFailed
          (if (Utilities|DoesObjectImplementInterface OtherActor "/Game/Interfaces/Spell.Spell_C")
            (if (== (Utilities|GetClass OtherActor) "/Game/Blueprints/BP_Door.BP_Door_C")
              (Actor|DestroyActor :!label _label)
              (else
                (bind _spellname (Class|Spell|UseSpell(Message) OtherActor (* (Math|Vector|GetForwardVector (Variables|/Script/Engine.MovementComponent|GetUpdatedPrimitive (Variables|Default|GetProjectileMovement))) 10000)))
                (Development|PrintString (Utilities|String|Append _spellname " Projectile to: " (Utilities|GetObjectName OtherActor)) true true "(R=0.497833,G=0.155935,B=0.526042,A=1.000000)")
                (Actor|DestroyActor)))
            (else
              (goto _label))))))))

(event Custom|DestroyInTime
  (Actor|DestroyActor))

(event EventBeginPlay
  (Utilities|Time|SetTimerbyEvent (delegate Custom|DestroyInTime) 15.0 true))

(fn ConstructionScript)