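; WinCondition tracks a set of pressure plates and signals the win door as open while all of them are active.
; On BeginPlay it binds handlers to each plate's activated and deactivated dispatchers, which raise or lower a shared count.
; Reaching the plate total turns the Cube green, and dropping one below it turns it red, each with a printed message; no door movement happens here.
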(event Custom|DeactivatedPlate
  (bind _count (Variables|Default|GetCount))
  (Math|Integer|DecrementInt _count
    (:%20%20
      (if (== _count (- (Utilities|Array|Length (Variables|Default|GetPlates)) 1))
        (Development|PrintString "Win Door Close" true true "(R=1.000000,G=0.000000,B=0.000000,A=1.000000)")
        (Rendering|Material|SetMaterial (Variables|Default|GetCube) 0 "/Game/Materials/Red.Red")))))

(event Custom|ActivatedPlate
  (bind _count (Variables|Default|GetCount))
  (Math|Integer|IncrementInt _count
    (:%20%20
      (if (>= _count (Utilities|Array|Length (Variables|Default|GetPlates)))
        (Development|PrintString "Win Door Open" true true "(R=0.000000,G=1.000000,B=0.000000,A=1.000000)")
        (Rendering|Material|SetMaterial (Variables|Default|GetCube) 0 "/Game/Materials/Green.Green")))))

(event EventBeginPlay
  (for _array_element (Variables|Default|GetPlates)
    (EventDispatchers|BindEventtoActivatedEventDispatcher _array_element (delegate Custom|ActivatedPlate))
    (EventDispatchers|BindEventtoDeactivatedEventDispatcher _array_element (delegate Custom|DeactivatedPlate))))

(fn ConstructionScript)