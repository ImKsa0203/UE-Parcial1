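; Damage zone that repeatedly damages anything inside its collider that has components implementing BPI_Damageable.
; Overlap begin and end events add and remove those components in a unique list.
; A looping timer calls Damage on every listed component each second, with a negative start delay making the first hit near-immediate.
; The timer starts with the first target and is cleared when the list empties.
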(event OnComponentBeginOverlap(DmgCollider)
  (params (OverlappedComponent :type Primitive%20Component%20Object%20Reference) (OtherActor :type Actor%20Object%20Reference) (OtherComp :type Primitive%20Component%20Object%20Reference) (OtherBodyIndex :type Integer) (bFromSweep :type Boolean) (SweepResult :type Hit%20Result%20Structure%20%28by%20ref%29))
  (for _array_element (Class|Actor|GetComponentsbyInterface OtherActor "/Game/Blueprints/ActorComponents/BPI_Damageable.BPI_Damageable_C")
    (bind _asbpi_damageable (Utilities|Casting|CastToBPI_Damageable _array_element))
    (Utilities|Array|AddUnique (Variables|Default|GetDamageable) _asbpi_damageable)
    (if (not (Utilities|Time|IsValidTimerHandle (Variables|Default|GetTimer)))
      (bind _returnvalue (Utilities|Time|SetTimerbyEvent (delegate Custom|DealDamage) 1.0 true -1.0))
      (Variables|Default|SetTimer _returnvalue))))

(event OnComponentEndOverlap(DmgCollider)
  (params (OverlappedComponent :type Primitive%20Component%20Object%20Reference) (OtherActor :type Actor%20Object%20Reference) (OtherComp :type Primitive%20Component%20Object%20Reference) (OtherBodyIndex :type Integer))
  (bind _damageable (Variables|Default|GetDamageable))
  (for _array_element (Class|Actor|GetComponentsbyInterface OtherActor "/Game/Blueprints/ActorComponents/BPI_Damageable.BPI_Damageable_C")
    (bind _asbpi_damageable (Utilities|Casting|CastToBPI_Damageable _array_element))
    (Utilities|Array|RemoveItem _damageable _asbpi_damageable)
    (if (Utilities|Array|IsEmpty _damageable)
      (Utilities|Time|ClearandInvalidateTimerbyHandle (Variables|Default|GetTimer)))))

(event Custom|DealDamage
  (for _array_element (Variables|Default|GetDamageable)
    (Default|Damage _array_element (Variables|Default|GetDamage))))

(fn ConstructionScript)