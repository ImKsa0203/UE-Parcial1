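; Actor component that tracks an actor's health, starting at MaxHealth on BeginPlay.
; Damage and Heal events route to TakeDamage and TakeHeal, which act only while the owner is alive; healing caps at MaxHealth, while damage has no lower clamp.
; Event dispatchers report damage, healing, health changes and death, alongside on-screen debug prints of health and death.
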(event EventBeginPlay
  (Variables|Default|SetHealth (Variables|Default|GetMaxHealth)))

(event EventHeal
  (params (Healing :type Float%20%28double-precision%29))
  (CallFunction|TakeHeal Healing))

(event EventDamage
  (params (Damage :type Float%20%28double-precision%29))
  (CallFunction|TakeDamage Damage))

(fn TakeDamage
  (params (Damage :type Float%20%28double-precision%29))
  (bind _maxhealth (Variables|Default|GetMaxHealth))
  (if (Utilities|IsAlive)
    (Variables|Default|SetHealth (- (Variables|Default|GetHealth) Damage))
    (Default|CallOnDamaged Damage)
    (Default|CallOnChangeHealth (Variables|Default|GetHealth) _maxhealth)
    (Development|PrintString (Utilities|String|Append "Health: " (Utilities|String|ToString(Float) (Variables|Default|GetHealth)) " / " (Utilities|String|ToString(Float) _maxhealth)) true true "(R=1.000000,G=1.000000,B=0.000000,A=1.000000)")
    (if (Utilities|IsDead)
      (Default|CallOnDeath)
      (Development|PrintString "Death" true true "(R=1.000000,G=0.470624,B=0.000000,A=1.000000)"))))

(fn TakeHeal
  (params (Healing :type Float%20%28double-precision%29))
  (bind _maxhealth (Variables|Default|GetMaxHealth))
  (if (Utilities|IsAlive)
    (Variables|Default|SetHealth (Math|Float|Min(Float) (+ (Variables|Default|GetHealth) Healing) (Variables|Default|GetMaxHealth)))
    (Default|CallOnHealed Healing)
    (Default|CallOnChangeHealth (Variables|Default|GetHealth) _maxhealth)
    (Development|PrintString (Utilities|String|Append "Health: " (Utilities|String|ToString(Float) (Variables|Default|GetHealth)) " / " (Utilities|String|ToString(Float) _maxhealth)) true true "(R=1.000000,G=1.000000,B=0.000000,A=1.000000)")))