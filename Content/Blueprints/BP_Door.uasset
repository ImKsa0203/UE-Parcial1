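; Door actor that toggles open and closed when interacted with or targeted by the Alohomora spell.
; Interact flips IsOpen, plays the matching sound and runs a Timeline forward to close or in reverse to open, lerping the Pivot's location and rotation.
; The construction script calls SetTime with a start value based on IsOpen.
; A widget labeled with the spell name is shown and hidden by ActivateSpell and DeactivateSpell.
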(event Custom|Interact
  (bind _pivot (Variables|Default|GetPivot))
  (bind _returnvalue (Transformation|GetWorldLocation _pivot))
  (Variables|Default|SetIsOpen (not (Variables|Default|GetIsOpen)))
  (if (Variables|Default|GetIsOpen)
    (Audio|SpawnSoundatLocation "/Game/Audio/SFX/Open_Door.Open_Door" _returnvalue "0, 0, 0" 1.0 1.0 0.0 0 0)
    (bind _lerp (Timeline|Timeline Reverse)
      (:Update
        (Transformation|SetRelativeLocationAndRotation (Variables|Default|GetPivot) (Math|Vector|Lerp(Vector) (Variables|Default|GetOpenPosition) (Variables|Default|GetClosePosition) _lerp) (Math|Rotator|Lerp(Rotator) (Variables|Default|GetOpenRotation) (Variables|Default|GetCloseRotation) _lerp) false false)))
    (else
      (Audio|SpawnSoundatLocation "/Game/Audio/SFX/Close_Door.Close_Door" _returnvalue "0, 0, 0" 1.0 1.0 0.0 0 0)
      (Timeline|Timeline Play))))

(event Custom|SetTime
  (params (NewTime :type Float%20%28single-precision%29))
  (bind _lerp (Timeline|Timeline SetNewTime)
    (:Update
      (Transformation|SetRelativeLocationAndRotation (Variables|Default|GetPivot) (Math|Vector|Lerp(Vector) (Variables|Default|GetOpenPosition) (Variables|Default|GetClosePosition) _lerp) (Math|Rotator|Lerp(Rotator) (Variables|Default|GetOpenRotation) (Variables|Default|GetCloseRotation) _lerp) false false))))

(event EventBeginPlay
  (bind _widget (Variables|Default|GetWidget))
  (bind _aswbp_spell_text (Utilities|Casting|CastToWBP_SpellText (UserInterface|GetWidget _widget)))
  (Rendering|Components|TextRender|SetText (Variables|/Game/Widgets/WBP_SpellText.WBP_SpellText_C|GetTextBlock _aswbp_spell_text) "Alohomora")
  (Rendering|SetVisibility _widget false false))

(event EventActivateSpell
  (Rendering|SetVisibility (Variables|Default|GetWidget) true false))

(event EventDeactivateSpell
  (Rendering|SetVisibility (Variables|Default|GetWidget) false false))

(fn ConstructionScript
  (CallFunction|SetTime (Math|Float|SelectFloat 0.0 1.0 (Variables|Default|GetIsOpen))))

(fn UseSpell
  (params (Direction :type Vector :default "0, 0, 0"))
  (CallFunction|Interact)
  (return "Alohomora"))